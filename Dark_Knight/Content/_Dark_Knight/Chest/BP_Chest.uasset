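; BP_Chest is an interactable chest that grants the player XP when opened.
; Its trigger sets a proximity flag and shows a Press E widget when the player overlaps, clearing both on exit.
; It binds to the player character's interaction event on BeginPlay, opening only while that flag is set.
; Opening starts the chest animation, adds XP and destroys the actor immediately, without waiting for the animation.
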(event `self.ReceiveBeginPlay`
  (bind _asbp_player_character (cast `/Game/_Dark_Knight/Blueprints/BP_PlayerCharacter` (`GameplayStatics.GetPlayerCharacter` 0)))
  (add `/Game/_Dark_Knight/Blueprints/BP_PlayerCharacter.UponInteraction` _asbp_player_character (delegate `Chest Open`)))

(event `Chest Open`
  (if (`self.IsPlayerNear?`)
    (`self.OpenThisChest`)))

(event `self.Trigger.OnComponentBeginOverlap`
  (params (OverlappedComponent :type "PrimitiveComponent Object Reference") (OtherActor :type "Actor Object Reference") (OtherComp :type "PrimitiveComponent Object Reference") (OtherBodyIndex :type Integer) (bFromSweep :type Boolean) (SweepResult :type "HitResult Structure (by ref)"))
  (cast `/Game/_Dark_Knight/Blueprints/BP_PlayerCharacter` OtherActor)
  (bind _returnvalue (`|CreateWidget` "/Game/_Dark_Knight/Widgets/PressE.PressE_C"))
  (`|ExecutionSequence`
    (:`then_0`
      (set `self.WGB_pressE` _returnvalue)
      (`UserWidget.AddToViewport` _returnvalue 0))
    (:`then_1`
      (set `self.IsPlayerNear?` true))))

(event `self.Trigger.OnComponentEndOverlap`
  (params (OverlappedComponent :type "PrimitiveComponent Object Reference") (OtherActor :type "Actor Object Reference") (OtherComp :type "PrimitiveComponent Object Reference") (OtherBodyIndex :type Integer))
  (`|ExecutionSequence`
    (:`then_0`
      (set `self.IsPlayerNear?` false))
    (:`then_1`
      (`Widget.RemoveFromParent` (`self.WGB_pressE`)))))

(fn `Open Chest`
  (returns (Item :type Boolean)))

(fn `OpenThisChest`
  (`SkeletalMeshComponent.PlayAnimation` (`self.Chest`) "/Game/_Dark_Knight/Chest/Chest_Open.Chest_Open" false)
  (bind _asbp_player_character (cast `/Game/_Dark_Knight/Blueprints/BP_PlayerCharacter` (`GameplayStatics.GetPlayerCharacter` 0)))
  (`/Game/_Dark_Knight/Blueprints/BP_PlayerCharacter.Increase XP` _asbp_player_character (`self.Added XP`))
  (`self.K2_DestroyActor`)
  (return))

(fn `UserConstructionScript`)