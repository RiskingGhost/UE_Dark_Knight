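; Lock-on targeting for the player character that keeps the camera and facing on a chosen target.
; Sphere trace gathers LockOnClass actors, then visibility traces and camera-forward dot products pick the most centred.
; A looping timer eases control rotation toward a point below the target, lowered with distance, and releases lock beyond LockOnRadius.
; Left/right switching selects the most centred other target, judging side by trace hit normal against camera right.
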(event `self.ReceiveBeginPlay`
  (set `self.PlayerReference` (cast `/Game/_Dark_Knight/Blueprints/BP_PlayerCharacter` (`GameplayStatics.GetPlayerCharacter` 0) :!pure true)))

(event `TriggerLockOn`
  (bind _targettolockon (`self.CheckClosestTarget` (`self.Find Target`)))
  (bind _charactermovement (`Character.CharacterMovement` (`self.PlayerReference`)))
  (`/Engine/EditorBlueprintResources/StandardMacros.IsValid` _targettolockon
    (:`Is Valid`
      (set `self.Target` _targettolockon)
      (set `self.isLockOn?` true)
      (set `CharacterMovementComponent.bOrientRotationToMovement` false _charactermovement)
      (set `CharacterMovementComponent.bUseControllerDesiredRotation` true _charactermovement)
      (`Controller.SetIgnoreLookInput` (`GameplayStatics.GetPlayerController` 0) true)
      (bind _returnvalue (`KismetSystemLibrary.K2_SetTimerDelegate` (delegate `TargetLockOn`) (`GameplayStatics.GetWorldDeltaSeconds`) true)))))

(event `EndLockOn`
  (bind _charactermovement (`Character.CharacterMovement` (`self.PlayerReference`)))
  (set `self.isLockOn?` false)
  (`KismetSystemLibrary.K2_ClearAndInvalidateTimerHandle` (stale `TriggerLockOn` _returnvalue))
  (set `CharacterMovementComponent.bOrientRotationToMovement` true _charactermovement)
  (set `CharacterMovementComponent.bUseControllerDesiredRotation` false _charactermovement)
  (`Controller.ResetIgnoreLookInput` (`GameplayStatics.GetPlayerController` 0)))

(event `TargetLockOn`
  (bind _returnvalue (`Pawn.GetController` (`self.PlayerReference`)))
  (bind _returnvalue_2 (`Controller.GetControlRotation` _returnvalue))
  (bind (_returnvalue_roll _returnvalue_pitch _returnvalue_yaw) (`KismetMathLibrary.BreakRotator` (`KismetMathLibrary.RInterpTo` _returnvalue_2 (`self.Locked Camara Movement`) 0.01 3.0)))
  (if (> (`KismetMathLibrary.Vector_Distance` (`Actor.K2_GetActorLocation` (`self.Target`)) (`Actor.K2_GetActorLocation` (`self.PlayerReference`))) (`self.LockOnRadius`))
    (`self.EndLockOn`)
    (else
      (`Controller.SetControlRotation` _returnvalue (`KismetMathLibrary.MakeRotator` (.roll _returnvalue_2) _returnvalue_pitch _returnvalue_yaw)))))

(event `Switch to Left`
  (`/Engine/EditorBlueprintResources/StandardMacros.IsValid` (`self.Target`)
    (:`Is Valid`
      (bind _newtarget (`self.GetTargetOnLeft`))
      (`/Engine/EditorBlueprintResources/StandardMacros.IsValid` _newtarget
        (:`Is Valid`
          (set `self.Target` _newtarget))))))

(event `Switch to Right`
  (`/Engine/EditorBlueprintResources/StandardMacros.IsValid` (`self.Target`)
    (:`Is Valid`
      (bind _newtarget (`self.GetTargetOnRight`))
      (`/Engine/EditorBlueprintResources/StandardMacros.IsValid` _newtarget
        (:`Is Valid`
          (set `self.Target` _newtarget))))))

(fn `CheckClosestTarget`
  (params (allTarget :type "Array of Actor Object Reference"))
  (returns (TargetToLockOn :type "Actor Object Reference"))
  (locals (CompareFloat :type "Float (double-precision)") (LockOnTarget :type "Actor Object Reference"))
  (for _array_element allTarget
    (bind (_outhit _returnvalue) (`KismetSystemLibrary.LineTraceSingle` (`SceneComponent.K2_GetComponentLocation` (`/Game/_Dark_Knight/Blueprints/BP_PlayerCharacter.FollowCamera` (`self.PlayerReference`))) (`Actor.K2_GetActorLocation` _array_element) "TraceTypeQuery1"))
    (if _returnvalue
      (if (`KismetMathLibrary.ClassIsChildOf` (`GameplayStatics.GetObjectClass` (`.HitActor` (`GameplayStatics.BreakHitResult` _outhit))) (`self.LockOnClass`))
        (bind _range (`self.CheckTargetAtCenter` _array_element))
        (`/Engine/EditorBlueprintResources/StandardMacros.CompareFloat` _range (`local.CompareFloat`)
          (:`>`
            (set `local.CompareFloat` _range)
            (set `local.LockOnTarget` _array_element))))))
  (return (`local.LockOnTarget`)))

(fn `CheckTargetAtCenter`
  (params (Target :type "Actor Object Reference"))
  (returns (Range :type "Float (double-precision)"))
  (bind _playerreference (`self.PlayerReference`))
  (return (`KismetMathLibrary.Dot_VectorVector` (`SceneComponent.GetForwardVector` (`/Game/_Dark_Knight/Blueprints/BP_PlayerCharacter.FollowCamera` _playerreference)) (`KismetMathLibrary.Conv_RotatorToVector` (`KismetMathLibrary.FindLookAtRotation` (`Actor.K2_GetActorLocation` _playerreference) (`Actor.K2_GetActorLocation` Target))))))

(fn `Find Target`
  (returns (Target :type "Array of Actor Object Reference"))
  (locals (LocalTarget :type "Array of Actor Object Reference"))
  (bind _localtarget (`local.LocalTarget`))
  (bind _returnvalue (`Actor.K2_GetActorLocation` (`self.PlayerReference`)))
  (bind (_outhits _returnvalue_2) (`KismetSystemLibrary.SphereTraceMultiForObjects` _returnvalue _returnvalue (`self.LockOnRadius`) (`|MakeArray` "ObjectTypeQuery7" :!type "EObjectTypeQuery Enum")))
  (if _returnvalue_2
    (for _array_element _outhits
      (bind (_bblockinghit _binitialoverlap _time _distance _location _impactpoint _normal _impactnormal _physmat _hitactor) (`GameplayStatics.BreakHitResult` _array_element))
      (if (`KismetMathLibrary.ClassIsChildOf` (`GameplayStatics.GetObjectClass` _hitactor) (`self.LockOnClass`))
        (`KismetArrayLibrary.Array_Add` _localtarget _hitactor)))
    (return _localtarget)))

(fn `GetTargetOnLeft`
  (returns (NewTarget :type "Actor Object Reference"))
  (locals (CompareFloat :type "Float (double-precision)") (LockOnTarget :type "Actor Object Reference"))
  (for _array_element (`self.Find Target`)
    (bind (_outhit _returnvalue) (`KismetSystemLibrary.LineTraceSingleForObjects` (`SceneComponent.K2_GetComponentLocation` (`/Game/_Dark_Knight/Blueprints/BP_PlayerCharacter.FollowCamera` (`self.PlayerReference`))) (`Actor.K2_GetActorLocation` _array_element) (`|MakeArray` "ObjectTypeQuery7" :!type "EObjectTypeQuery Enum")))
    (if _returnvalue
      (if (and (!= (`self.Target`) _array_element) (> (`KismetMathLibrary.DegAsin` (`KismetMathLibrary.Dot_VectorVector` (`SceneComponent.GetRightVector` (`/Game/_Dark_Knight/Blueprints/BP_PlayerCharacter.FollowCamera` (`self.PlayerReference`))) (`.Normal` (`GameplayStatics.BreakHitResult` _outhit)))) 0.0))
        (bind _range (`self.CheckTargetAtCenter` _array_element))
        (`/Engine/EditorBlueprintResources/StandardMacros.CompareFloat` _range (`local.CompareFloat`)
          (:`>`
            (set `local.CompareFloat` _range)
            (set `local.LockOnTarget` _array_element))))))
  (return (`local.LockOnTarget`)))

(fn `GetTargetOnRight`
  (returns (NewTarget :type "Actor Object Reference"))
  (locals (CompareFloat :type "Float (double-precision)") (LockOnTarget :type "Actor Object Reference"))
  (for _array_element (`self.Find Target`)
    (bind (_outhit _returnvalue) (`KismetSystemLibrary.LineTraceSingleForObjects` (`SceneComponent.K2_GetComponentLocation` (`/Game/_Dark_Knight/Blueprints/BP_PlayerCharacter.FollowCamera` (`self.PlayerReference`))) (`Actor.K2_GetActorLocation` _array_element) (`|MakeArray` "ObjectTypeQuery7" :!type "EObjectTypeQuery Enum")))
    (if _returnvalue
      (if (and (!= (`self.Target`) _array_element) (< (`KismetMathLibrary.DegAsin` (`KismetMathLibrary.Dot_VectorVector` (`SceneComponent.GetRightVector` (`/Game/_Dark_Knight/Blueprints/BP_PlayerCharacter.FollowCamera` (`self.PlayerReference`))) (`.Normal` (`GameplayStatics.BreakHitResult` _outhit)))) 0.0))
        (bind _range (`self.CheckTargetAtCenter` _array_element))
        (`/Engine/EditorBlueprintResources/StandardMacros.CompareFloat` _range (`local.CompareFloat`)
          (:`>`
            (set `local.CompareFloat` _range)
            (set `local.LockOnTarget` _array_element))))))
  (return (`local.LockOnTarget`)))

(fn `Locked Camara Movement`
  (returns (ReturnValue :type "Rotator Structure"))
  (bind _playerreference (`self.PlayerReference`))
  (bind _target (`self.Target`))
  (bind (_returnvalue_x _returnvalue_y _returnvalue_z) (`KismetMathLibrary.BreakVector` (`Actor.K2_GetActorLocation` _target)))
  (return (`KismetMathLibrary.FindLookAtRotation` (`SceneComponent.K2_GetComponentLocation` (`/Game/_Dark_Knight/Blueprints/BP_PlayerCharacter.FollowCamera` _playerreference)) (`KismetMathLibrary.MakeVector` _returnvalue_x _returnvalue_y (- _returnvalue_z (/ (`KismetMathLibrary.Vector_Distance` (`Actor.K2_GetActorLocation` _playerreference) (`Actor.K2_GetActorLocation` _target)) 5.0))))))