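; BP_UpgradeBonfire is an interactable bonfire that opens the BonfireMenu widget when the player interacts nearby.
; Overlap tracks proximity, shows a PressE prompt, registers the bonfire on BP_PlayerCharacter and grants XP on each player entry.
; The player's interaction event opens the menu, switches to UI-only input with a cursor and disables sphere collision.
; LeaveButton closes the menu and restores game input and query collision.
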(event `self.ReceiveBeginPlay`
  (bind _asbp_player_character (cast `/Game/_Dark_Knight/Blueprints/BP_PlayerCharacter` (`GameplayStatics.GetPlayerCharacter` 0)))
  (`KismetSystemLibrary.PrintString` "done")
  (add `/Game/_Dark_Knight/Blueprints/BP_PlayerCharacter.UponInteraction` _asbp_player_character (delegate `OpenBonfire`))
  (bind _returnvalue (`|CreateWidget` "/Game/_Dark_Knight/Widgets/PressE.PressE_C"))
  (set `self.WGB_pressE` _returnvalue))

(event `OpenBonfire`
  (if (`self.IsPlayerNear?`)
    (`self.UseBonfire`)))

(event `self.ReceiveActorBeginOverlap`
  (params (OtherActor :type "Actor Object Reference"))
  (set `self.IsPlayerNear?` true)
  (bind _asbp_player_character (cast `/Game/_Dark_Knight/Blueprints/BP_PlayerCharacter` OtherActor))
  (set `/Game/_Dark_Knight/Blueprints/BP_PlayerCharacter.Bonfire Ref` self _asbp_player_character)
  (`UserWidget.AddToViewport` (`self.WGB_pressE`) 0)
  (`/Game/_Dark_Knight/Blueprints/BP_PlayerCharacter.Increase XP` _asbp_player_character 100))

(event `self.ReceiveActorEndOverlap`
  (params (OtherActor :type "Actor Object Reference"))
  (set `self.IsPlayerNear?` false)
  (`Widget.RemoveFromParent` (`self.WGB_pressE`)))

(event `UseBonfire`
  (bind _returnvalue (`GameplayStatics.GetPlayerController` 0))
  (`KismetSystemLibrary.PrintString` "Bonfire Menu open")
  (`Widget.RemoveFromParent` (`self.WGB_pressE`))
  (bind _returnvalue_2 (`|CreateWidget` "/Game/_Dark_Knight/Widgets/BonfireMenu.BonfireMenu_C"))
  (bind _output_get (set `self.WGB_BonfireMenu` _returnvalue_2))
  (`UserWidget.AddToViewport` _output_get 0)
  (`WidgetBlueprintLibrary.SetInputMode_UIOnlyEx` _returnvalue (`/Game/_Dark_Knight/Widgets/BonfireMenu.Leave_Btn` (`self.WGB_BonfireMenu`)))
  (set `PlayerController.bShowMouseCursor` true _returnvalue)
  (add `/Game/_Dark_Knight/Widgets/BonfireMenu.OnPressLeave` (`self.WGB_BonfireMenu`) (`|CreateDelegate` :!event `LeaveButton`))
  (`PrimitiveComponent.SetCollisionEnabled` (`self.Sphere`) "NoCollision"))

(event `LeaveButton`
  (bind _returnvalue (`GameplayStatics.GetPlayerController` 0))
  (`Widget.RemoveFromParent` (`self.WGB_BonfireMenu`))
  (set `self.WGB_BonfireMenu` null)
  (`WidgetBlueprintLibrary.SetInputMode_GameOnly` _returnvalue)
  (set `PlayerController.bShowMouseCursor` false _returnvalue)
  (`PrimitiveComponent.SetCollisionEnabled` (`self.Sphere`) "QueryOnly"))

(fn `UserConstructionScript`)