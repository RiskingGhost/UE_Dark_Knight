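; BP_UpgradeBonfire is a bonfire actor that shows an interaction prompt when the player comes near.
; Overlap by BP_ThirdPersonCharacter creates a PressE widget, adds it to the viewport and sets IsPlayerNear.
; End overlap clears the flag and removes the widget, without checking which actor left.
; No input handling or upgrade logic is in this graph, and the flag is only written here.
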(event `self.ReceiveActorBeginOverlap`
  (params (OtherActor :type "Actor Object Reference"))
  (cast `/Game/ThirdPerson/Blueprints/BP_ThirdPersonCharacter` OtherActor)
  (bind _returnvalue (`|CreateWidget` "/Game/_Dark_Knight/Widgets/PressE.PressE_C"))
  (`|ExecutionSequence`
    (:`then_0`
      (set `self.WGB_pressE` _returnvalue)
      (`UserWidget.AddToViewport` _returnvalue 0))
    (:`then_1`
      (set `self.IsPlayerNear?` true))))

(event `self.ReceiveActorEndOverlap`
  (params (OtherActor :type "Actor Object Reference"))
  (`|ExecutionSequence`
    (:`then_0`
      (set `self.IsPlayerNear?` false))
    (:`then_1`
      (`Widget.RemoveFromParent` (`self.WGB_pressE`)))))

(fn `UserConstructionScript`)